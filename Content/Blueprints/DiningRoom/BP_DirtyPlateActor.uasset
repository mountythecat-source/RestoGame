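; Dirty plate actor for the dining room that is cleaned through interaction and destroys itself when done.
; Interactable hides the CleanTimer widget component, caches its WB_ProgressTimer and sets a timer on UpdateClean.
; UpdateClean subtracts CleaningTimer from CurrentTime, updates the progress widget, and at zero clears the timer and destroys the plate.
; TimeToClean holds an unfinished copy of this logic, with unconnected nodes.
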(event `/Game/ThirdPerson/Blueprints/BPI_Interactable.Interactable`
  (params (Player :type "/Game/ThirdPerson/Blueprints/BP_ThirdPersonCharacter Object Reference"))
  (`SceneComponent.SetVisibility` (`self.CleanTimer`) false false)
  (bind _aswb_progress_timer (cast `/Game/UI/WB_ProgressTimer` (`WidgetComponent.GetWidget` (`self.CleanTimer`))))
  (set `self.WB_CleanTimer` _aswb_progress_timer)
  (bind _returnvalue (`KismetSystemLibrary.K2_SetTimerDelegate` (delegate `UpdateClean`) (`self.CleaningTimer`))))

(event `UpdateClean`
  (bind _output_get (set `self.CurrentTime` (- (`self.CurrentTime`) (`self.CleaningTimer`))))
  (`/Game/UI/WB_ProgressTimer.Update Timer` (`self.WB_CleanTimer`) _output_get (`self.MaxTimer`))
  (if (<= (`self.CurrentTime`) 0.0)
    (`SceneComponent.SetVisibility` (`self.CleanTimer`) false false)
    (`KismetSystemLibrary.K2_ClearAndInvalidateTimerHandle` (stale `/Game/ThirdPerson/Blueprints/BPI_Interactable.Interactable` _returnvalue))
    (set `self.CurrentTime` (`self.MaxTimer`))
    (`self.K2_DestroyActor`)))

(fn `NewFunction`)

(fn `TimeToClean`
  (bind _aswb_progress_timer (cast `/Game/UI/WB_ProgressTimer` _))
  (set `self.WB_CleanTimer` _aswb_progress_timer)
  (bind _returnvalue (`KismetSystemLibrary.K2_SetTimerDelegate` :`Time` (`self.CleaningTimer`))))

(fn `UserConstructionScript`)