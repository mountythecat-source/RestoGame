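; BP_Table is an interactable dining table that seats customer NPCs and takes delivery of their orders.
; Interacting with a clean, free table seats the player's selected NPC, rolls a random menu order and announces it through the player controller's MenuChoice.
; Serving matching held food completes the order, destroys the food, spawns a dirty plate and marks the table unclean.
; RemoveNPC frees the seat.
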(event `self.ReceiveActorBeginOverlap`
  (params (OtherActor :type "Actor Object Reference")))

(event `self.ReceiveBeginPlay`)

(event `/Game/ThirdPerson/Blueprints/BPI_Interactable.Interactable`
  (params (Player :type "/Game/ThirdPerson/Blueprints/BP_ThirdPersonCharacter Object Reference"))
  (bind _heldingredientactor (`/Game/ThirdPerson/Blueprints/BP_ThirdPersonCharacter.HeldIngredientActor` Player))
  (bind _selectednpc (`/Game/ThirdPerson/Blueprints/BP_ThirdPersonCharacter.SelectedNPC` Player))
  (if (`self.IsOccupied?`)
    (if (`KismetSystemLibrary.IsValid` _heldingredientactor)
      (bind _asbp_food (cast `/Game/Blueprints/Kitchen/BP_Food` _heldingredientactor))
      (bind _ecurrentfood (`/Game/Blueprints/Kitchen/BP_Food.GetMenu` _asbp_food))
      (if (`|EnumEquality` _ecurrentfood (`self.CurrentOrder`))
        (`self.Order Complete` Player)
        (bind _returnvalue (`|SpawnActorFromClass` "/Game/Blueprints/DiningRoom/BP_DirtyPlateActor.BP_DirtyPlateActor_C" (`self.GetTransform`) "Undefined" "MultiplyWithRoot" null self null))
        (`self.K2_SetActorLocation` _returnvalue (`SceneComponent.K2_GetComponentLocation` (`self.DirtPoint`)) false false)
        (set `self.IsCleaned?` false)))
    (elif (`self.IsCleaned?`)
      (`/Engine/EditorBlueprintResources/StandardMacros.IsValid` _selectednpc
        (:`Is Valid`
          (bind _output_get (set `self.AssignedNPC` _selectednpc))
          (`self.K2_SetActorLocation` _output_get (`SceneComponent.K2_GetComponentLocation` (`self.StandPoint`)) false true)
          (`/Game/Blueprints/NPC/BP_NPC.Set Table` _selectednpc self)
          (`self.The NPC Sits` self))
        (:`Is Not Valid`
          (`KismetSystemLibrary.PrintString` "Dude There's already a dude..."))))))

(event `The NPC Sits`
  (bind _asbp_third_person_player_controller (cast `/Game/ThirdPerson/Blueprints/BP_ThirdPersonPlayerController` (`GameplayStatics.GetPlayerController` 0)))
  (set `self.IsOccupied?` true)
  (bind _output_get (set `self.CurrentOrder` (select `int` (`KismetMathLibrary.RandomIntegerInRange` 0 5) :`0` "NewEnumerator0" :`1` "NewEnumerator1" :`2` "NewEnumerator2" :`3` "NewEnumerator3" :`4` "NewEnumerator4" :!type "/Game/UI/EMenu Enum")))
  (`KismetSystemLibrary.PrintString` (`|GetEnumeratorNameAsString` _output_get))
  (message `/Game/ThirdPerson/Blueprints/BPI_TheOrderUI.NotifyOrderCreated` (`/Game/ThirdPerson/Blueprints/BP_ThirdPersonPlayerController.Menu Choice` _asbp_third_person_player_controller) (`self.TableID`) _output_get "" null)
  (`/Game/Blueprints/NPC/BP_NPC.Sit in table` (`self.AssignedNPC`)))

(event `Remove NPC`
  (`/Engine/EditorBlueprintResources/StandardMacros.IsValid` (`self.AssignedNPC`)
    (:`Is Valid`
      (set `self.AssignedNPC` null)
      (set `self.IsOccupied?` false))))

(event `Order Complete`
  (params (Player :type "/Game/ThirdPerson/Blueprints/BP_ThirdPersonCharacter Object Reference"))
  (`/Game/Blueprints/NPC/BP_NPC.Finish Order` (`self.AssignedNPC`) true (`self.TableID`))
  (`self.K2_DestroyActor` (`/Game/ThirdPerson/Blueprints/BP_ThirdPersonCharacter.HeldIngredientActor` Player))
  (set `/Game/ThirdPerson/Blueprints/BP_ThirdPersonCharacter.HeldIngredientActor` null Player))

(fn `UserConstructionScript`)