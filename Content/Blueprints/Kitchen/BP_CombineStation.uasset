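; Kitchen station that combines two ingredients carried by the player into prepared food.
; On interact, held ingredients fill slot A, then B (both attach to SlotBPoint), recording their types and triggering CombineFood once B fills.
; Either of two order-independent recipes spawns a BP_PreparedFood on the player's chest hold point; other pairs are simply destroyed.
; An older, unconnected version of this logic remains in the graph.
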(event `CombineFood`
  (if (or (and (`|EnumEquality` (`self.IngredientA`) "NewEnumerator0") (`|EnumEquality` (`self.IngredientB`) "NewEnumerator1")) (and (`|EnumEquality` (`self.IngredientA`) "NewEnumerator1") (`|EnumEquality` (`self.IngredientB`) "NewEnumerator0")))
    (`self.DestroySlotASlotB`)
    (bind _returnvalue (`|SpawnActorFromClass` "/Game/Blueprints/Kitchen/BP_PreparedFood.BP_PreparedFood_C" (`KismetMathLibrary.Conv_VectorToTransform` (`SceneComponent.K2_GetComponentLocation` (`self.Box`))) "Undefined" "MultiplyWithRoot" null "NewEnumerator0" "NewEnumerator1" null))
    (bind _output_get (set `self.PreparedFood` _returnvalue))
    (set `/Game/ThirdPerson/Blueprints/BP_ThirdPersonCharacter.HeldIngredientActor` _output_get (stale `/Game/ThirdPerson/Blueprints/BPI_Interactable.Interactable` Player))
    (bind _chestholdpoint (`/Game/ThirdPerson/Blueprints/BP_ThirdPersonCharacter.ChestHoldPoint` (stale `/Game/ThirdPerson/Blueprints/BPI_Interactable.Interactable` Player)))
    (`self.K2_AttachToComponent` _output_get _chestholdpoint "None" "SnapToTarget" "KeepRelative" "KeepWorld" true)
    (elif (or (and (`|EnumEquality` (`self.IngredientA`) "NewEnumerator0") (`|EnumEquality` (`self.IngredientB`) "NewEnumerator2")) (and (`|EnumEquality` (`self.IngredientA`) "NewEnumerator2") (`|EnumEquality` (`self.IngredientB`) "NewEnumerator0")))
      (`self.DestroySlotASlotB`)
      (bind _returnvalue_2 (`|SpawnActorFromClass` "/Game/Blueprints/Kitchen/BP_PreparedFood.BP_PreparedFood_C" (`KismetMathLibrary.Conv_VectorToTransform` (`SceneComponent.K2_GetComponentLocation` (`self.Box`))) "Undefined" "MultiplyWithRoot" null "NewEnumerator1" "NewEnumerator1" null))
      (bind _output_get_2 (set `self.PreparedFood` _returnvalue_2))
      (set `/Game/ThirdPerson/Blueprints/BP_ThirdPersonCharacter.HeldIngredientActor` _output_get_2 (stale `/Game/ThirdPerson/Blueprints/BPI_Interactable.Interactable` Player))
      (`self.K2_AttachToComponent` _output_get_2 _chestholdpoint "None" "SnapToTarget" "KeepRelative" "KeepWorld" true)
      (else
        (`self.DestroySlotASlotB`)))))

(event `DestroySlotASlotB`
  (`self.K2_DestroyActor` (`self.SlotAIngredient`))
  (`self.K2_DestroyActor` (`self.SlotBIngredient`))
  (set `self.SlotAIngredient` null)
  (set `self.SlotBIngredient` null)
  (set `/Game/ThirdPerson/Blueprints/BP_ThirdPersonCharacter.HeldIngredientActor` null (stale `/Game/ThirdPerson/Blueprints/BPI_Interactable.Interactable` Player)))

(event `SetIngredeintSlotB`
  (bind _ingredienttype (message `/Game/ThirdPerson/Blueprints/BPI_Carriable.GetIngredientType` (`/Game/ThirdPerson/Blueprints/BP_ThirdPersonCharacter.HeldIngredientActor` (stale `/Game/ThirdPerson/Blueprints/BPI_Interactable.Interactable` Player))))
  (set `self.IngredientB` _ingredienttype))

(event `SetIngredeintSlotA`
  (bind _ingredienttype (message `/Game/ThirdPerson/Blueprints/BPI_Carriable.GetIngredientType` (`/Game/ThirdPerson/Blueprints/BP_ThirdPersonCharacter.HeldIngredientActor` (stale `/Game/ThirdPerson/Blueprints/BPI_Interactable.Interactable` Player))))
  (set `self.IngredientA` _ingredienttype))

(event `/Game/ThirdPerson/Blueprints/BPI_Interactable.Interactable`
  (params (Player :type "/Game/ThirdPerson/Blueprints/BP_ThirdPersonCharacter Object Reference"))
  (bind _heldingredientactor (`/Game/ThirdPerson/Blueprints/BP_ThirdPersonCharacter.HeldIngredientActor` Player))
  (bind _eitemcategory (message `/Game/ThirdPerson/Blueprints/BPI_Carriable.GetItemType` _heldingredientactor))
  (switch `/Game/UI/EItemCategory` _eitemcategory
    (:`NewEnumerator0`
      (`/Engine/EditorBlueprintResources/StandardMacros.IsValid` _heldingredientactor
        (:`Is Valid`
          (if (`KismetSystemLibrary.IsValid` (`self.SlotAIngredient`))
            (if (not (`KismetSystemLibrary.IsValid` (`self.SlotBIngredient`)))
              (bind _output_get (set `self.SlotBIngredient` _heldingredientactor))
              (`self.K2_AttachToComponent` _output_get (`self.SlotBPoint`) "None" "SnapToTarget" "KeepRelative" "KeepWorld" true)
              (`self.SetIngredeintSlotB`)
              (set `/Game/ThirdPerson/Blueprints/BP_ThirdPersonCharacter.HeldIngredientActor` null Player)
              (`self.CombineFood`))
            (else
              (bind _output_get_2 (set `self.SlotAIngredient` _heldingredientactor))
              (`self.K2_AttachToComponent` _output_get_2 (`self.SlotBPoint`) "None" "SnapToTarget" "KeepRelative" "KeepWorld" true)
              (`self.SetIngredeintSlotA`)
              (set `/Game/ThirdPerson/Blueprints/BP_ThirdPersonCharacter.HeldIngredientActor` null Player))))))))

(fn `GetIngredientType`
  (returns (IngredientType :type "/Game/UI/EIngredient Enum"))
  (return "NewEnumerator0"))

(fn `GetItemType`
  (returns (EItemCategory :type "/Game/UI/EItemCategory Enum"))
  (return "NewEnumerator0"))

(fn `GetPreparedFood`
  (returns (PreparedFood :type "/Game/UI/EPreparedFood Enum"))
  (return "NewEnumerator0"))

(fn `UserConstructionScript`)