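; BP_Ingredient is a kitchen ingredient actor that a player can pick up, carry and drop.
; Its Interactable event checks the player's HeldIngredientActor before picking up, then stores itself there.
; Pickup disables collision and snaps the actor to the player's ChestHoldPoint; OnDropped detaches it, places it at the supplied transform and restores collision.
; GetIngredientType exposes the ingredient's type to other objects.
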(event `/Game/ThirdPerson/Blueprints/BPI_Carriable.OnDropped`
  (params (DropTransform :type "Transform Structure"))
  (`self.K2_DetachFromActor` "KeepWorld" "KeepWorld" "KeepWorld")
  (`self.K2_SetActorTransform` DropTransform)
  (`self.SetActorEnableCollision` true))

(event `/Game/ThirdPerson/Blueprints/BPI_Carriable.OnPickedUp`
  (params (Player :type "/Game/ThirdPerson/Blueprints/BP_ThirdPersonCharacter Object Reference"))
  (`self.SetActorEnableCollision` false)
  (`self.K2_AttachToComponent` (`/Game/ThirdPerson/Blueprints/BP_ThirdPersonCharacter.ChestHoldPoint` Player) "None" "SnapToTarget" "SnapToTarget" "KeepWorld" false))

(event `/Game/ThirdPerson/Blueprints/BPI_Interactable.Interactable`
  (params (Player :type "/Game/ThirdPerson/Blueprints/BP_ThirdPersonCharacter Object Reference"))
  (if (== (`/Game/ThirdPerson/Blueprints/BP_ThirdPersonCharacter.HeldIngredientActor` Player) null)
    (`self.OnPickedUp` Player)
    (set `/Game/ThirdPerson/Blueprints/BP_ThirdPersonCharacter.HeldIngredientActor` self Player)))

(fn `GetIngredientType`
  (returns (IngredientType :type "/Game/UI/EIngredient Enum"))
  (return (`self.IngredientType`)))

(fn `UserConstructionScript`)