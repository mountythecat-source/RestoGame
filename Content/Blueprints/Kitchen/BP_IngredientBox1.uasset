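; BP_IngredientBox1 is a kitchen dispenser, unlockable during play, that hands the player a new ingredient.
; While locked at BeginPlay, the Box component is invisible and both boxes lack collision; Unlocked restores them.
; Interactable spawns a BP_Ingredient at SpawnPoint, sets its type and mesh, then attaches it collision-free to the player's ChestHoldPoint as the held ingredient.
; The three type getters return fixed enum values, independent of IngredientToSpawn.
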(event `self.ReceiveBeginPlay`
  (if (not (`self.IsUnlocked?`))
    (`self.SetActorHiddenInGame` false)
    (`PrimitiveComponent.SetCollisionEnabled` (`self.Box1`) "NoCollision")
    (`SceneComponent.SetVisibility` (`self.Box`) false false)
    (`PrimitiveComponent.SetCollisionEnabled` (`self.Box`) "NoCollision")))

(event `Unlocked`
  (set `self.IsUnlocked?` true)
  (`self.SetActorHiddenInGame` false)
  (`PrimitiveComponent.SetCollisionEnabled` (`self.Box1`) "QueryAndPhysics")
  (`SceneComponent.SetVisibility` (`self.Box`) true false)
  (`PrimitiveComponent.SetCollisionEnabled` (`self.Box`) "QueryAndPhysics"))

(event `/Game/ThirdPerson/Blueprints/BPI_Interactable.Interactable`
  (params (Player :type "/Game/ThirdPerson/Blueprints/BP_ThirdPersonCharacter Object Reference"))
  (bind _returnvalue (`|SpawnActorFromClass` "/Game/Blueprints/Kitchen/BP_Ingredient.BP_Ingredient_C" (`SceneComponent.K2_GetComponentToWorld` (`self.SpawnPoint`)) "AlwaysSpawn" "MultiplyWithRoot" null null))
  (set `/Game/Blueprints/Kitchen/BP_Ingredient.IngredientType` (`self.IngredientToSpawn`) _returnvalue)
  (`StaticMeshComponent.SetStaticMesh` (`/Game/Blueprints/Kitchen/BP_Ingredient.StaticMesh` _returnvalue) (`self.New Mesh`))
  (set `/Game/ThirdPerson/Blueprints/BP_ThirdPersonCharacter.HeldIngredientActor` _returnvalue Player)
  (`self.OnPickedUp` Player))

(event `/Game/ThirdPerson/Blueprints/BPI_Carriable.OnPickedUp`
  (params (Player :type "/Game/ThirdPerson/Blueprints/BP_ThirdPersonCharacter Object Reference"))
  (bind _heldingredientactor (`/Game/ThirdPerson/Blueprints/BP_ThirdPersonCharacter.HeldIngredientActor` Player))
  (`self.SetActorEnableCollision` _heldingredientactor false)
  (`self.K2_AttachToComponent` _heldingredientactor (`/Game/ThirdPerson/Blueprints/BP_ThirdPersonCharacter.ChestHoldPoint` Player) "None" "SnapToTarget" "SnapToTarget" "KeepWorld" false))

(fn `GetIngredientType`
  (returns (IngredientType :type "/Game/UI/EIngredient Enum"))
  (return "NewEnumerator0"))

(fn `GetItemType`
  (returns (EItemCategory :type "/Game/UI/EItemCategory Enum"))
  (return "NewEnumerator0"))

(fn `GetPreparedFood`
  (returns (PreparedFood :type "/Game/UI/EPreparedFood Enum"))
  (return "NewEnumerator0"))

(fn `UserConstructionScript`)