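; Kitchen oven station meant to turn a player's held prepared food into a finished BP_Food dish.
; On interaction it reads the held item through message calls, records the prepared type, destroys the item and shows PreFoodPoint.
; FinishCooking spawns BP_Food with the matching menu and destroys the cooked input.
; The code that sets CookedFood and starts the FinishCooking timer is disconnected, so interacting never produces a dish.
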(event `Finish Cooking`
  (set `self.IsCooking?` false)
  (bind _returnvalue (`|SpawnActorFromClass` "/Game/Blueprints/Kitchen/BP_Food.BP_Food_C" (`KismetMathLibrary.MakeTransform` (0.0 0.0 0.0)) "Undefined" "MultiplyWithRoot" null null))
  (switch `/Game/UI/EPreparedFood` (`/Game/Blueprints/Kitchen/BP_PreparedFood.PreparedType` (`self.Cooked Food`))
    (:`NewEnumerator0`
      (set `/Game/Blueprints/Kitchen/BP_Food.Menu` "NewEnumerator0" _returnvalue))
    (:`NewEnumerator1`
      (set `/Game/Blueprints/Kitchen/BP_Food.Menu` "NewEnumerator1" _returnvalue)))
  (message `/Game/ThirdPerson/Blueprints/BPI_Carriable.OnPickedUp` _returnvalue null)
  (`self.K2_DestroyActor` (`self.Cooked Food`))
  (set `self.Cooked Food` null))

(event `/Game/ThirdPerson/Blueprints/BPI_Interactable.Interactable`
  (params (Player :type "/Game/ThirdPerson/Blueprints/BP_ThirdPersonCharacter Object Reference"))
  (bind _heldingredientactor (`/Game/ThirdPerson/Blueprints/BP_ThirdPersonCharacter.HeldIngredientActor` Player))
  (bind _eitemcategory (message `/Game/ThirdPerson/Blueprints/BPI_Carriable.GetItemType` _heldingredientactor))
  (switch `/Game/UI/EItemCategory` _eitemcategory
    (:`NewEnumerator1`
      (bind _preparedfood (message `/Game/ThirdPerson/Blueprints/BPI_Carriable.GetPreparedFood` _heldingredientactor))
      (bind _output_get (set `self.E PreparedFood` _preparedfood))
      (switch `/Game/UI/EPreparedFood` _output_get
        (:`NewEnumerator0`
          _)
        (:`NewEnumerator1`
          _))
      (`/Engine/EditorBlueprintResources/StandardMacros.IsValid` _heldingredientactor
        (:`Is Valid`
          (`self.K2_DestroyActor` _heldingredientactor)
          (set `/Game/ThirdPerson/Blueprints/BP_ThirdPersonCharacter.HeldIngredientActor` null Player)
          (`SceneComponent.SetVisibility` (`self.PreFoodPoint`) true false))))))

(fn `UserConstructionScript`)