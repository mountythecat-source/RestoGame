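; BP_PreparedFood is a kitchen item actor representing a prepared menu dish that can be dropped into the world.
; OnDropped detaches it, applies the drop transform and re-enables collision.
; Getters expose its item type and prepared type, while the ingredient type getter returns a fixed enum value.
; OnPickedUp, Interactable and BeginPlay are empty, with chest-attach pickup and per-menu sphere material logic left unconnected.
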(event `self.ReceiveBeginPlay`)

(event `/Game/ThirdPerson/Blueprints/BPI_Carriable.OnPickedUp`
  (params (Player :type "/Game/ThirdPerson/Blueprints/BP_ThirdPersonCharacter Object Reference")))

(event `/Game/ThirdPerson/Blueprints/BPI_Carriable.OnDropped`
  (params (DropTransform :type "Transform Structure"))
  (`self.K2_DetachFromActor` "KeepWorld" "KeepWorld" "KeepWorld")
  (`self.K2_SetActorTransform` DropTransform)
  (`self.SetActorEnableCollision` true))

(event `/Game/ThirdPerson/Blueprints/BPI_Interactable.Interactable`
  (params (Player :type "/Game/ThirdPerson/Blueprints/BP_ThirdPersonCharacter Object Reference")))

(fn `GetIngredientType`
  (returns (IngredientType :type "/Game/UI/EIngredient Enum"))
  (return "NewEnumerator0"))

(fn `GetItemType`
  (returns (EItemCategory :type "/Game/UI/EItemCategory Enum"))
  (return (`self.EItem`)))

(fn `GetPreparedFood`
  (returns (PreparedFood :type "/Game/UI/EPreparedFood Enum"))
  (return (`self.PreparedType`)))

(fn `UserConstructionScript`)