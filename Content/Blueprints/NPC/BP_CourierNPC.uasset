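; Courier NPC Blueprint that stands at a pick-up window and takes part in the order flow of its parent NPC class.
; On BeginPlay it attaches to the PickUpWindow's StandPoint, snapping location while keeping relative rotation and world scale, then runs parent startup.
; Interaction and order completion defer to the parent, with FinishOrder passing the success flag and a fixed table ID of zero.
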(event `self.ReceiveTick`
  (params (DeltaSeconds :type "Float (single-precision)"))
  (`parent.ReceiveTick` DeltaSeconds))

(event `self.ReceiveBeginPlay`
  (`self.K2_AttachToComponent` (`/Game/Blueprints/DiningRoom/BP_Table.StandPoint` (`self.Pick up Window`)) "None" "SnapToTarget" "KeepRelative" "KeepWorld")
  (`parent.ReceiveBeginPlay`))

(event `/Game/ThirdPerson/Blueprints/BPI_Interactable.Interactable`
  (params (Player :type "/Game/ThirdPerson/Blueprints/BP_ThirdPersonCharacter Object Reference"))
  (`parent.Interactable` null))

(event `self.Finish Order`
  (params (IsSucess :type Boolean) (TableId :type Integer))
  (`parent.Finish Order` IsSucess 0))

(fn `UserConstructionScript`
  (`parent.UserConstructionScript`))