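; BP_NPCSpawner periodically spawns BP_NPC actors inside its box area while the game mode's StatusStore flag is true.
; A looping BeginPlay timer checks the CurrentNPCS cap, then spawns at a random X/Y in the box with a random NPCData entry.
; The count only increments; UnregisterNPC removes the NPC's class from ActiveNPCs, which is never filled here, and leaves CurrentNPCS unchanged.
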(event `self.ReceiveBeginPlay`
  (`KismetSystemLibrary.K2_SetTimerDelegate` (delegate `Spawn NPC`) 10.0 true))

(event `Spawn NPC`
  (bind _box (`self.Box`))
  (bind (_returnvalue_x _returnvalue_y) (`KismetMathLibrary.BreakVector` (`KismetMathLibrary.RandomPointInBoundingBox` (`SceneComponent.K2_GetComponentLocation` _box) (`BoxComponent.GetScaledBoxExtent` _box))))
  (bind _asbp_third_person_game_mode (cast `/Game/ThirdPerson/Blueprints/BP_ThirdPersonGameMode` (`GameplayStatics.GetGameMode`)))
  (if (`/Game/ThirdPerson/Blueprints/BP_ThirdPersonGameMode.Status store` _asbp_third_person_game_mode)
    (if (< (`self.Current NPCS`) (`self.Max NPCS`))
      (`|SpawnActorFromClass` "/Game/Blueprints/NPC/BP_NPC.BP_NPC_C" (`KismetMathLibrary.MakeTransform` (`KismetMathLibrary.MakeVector` _returnvalue_x _returnvalue_y) (struct :`Yaw` 180.0)) "Undefined" "MultiplyWithRoot" null (`|GetArrayItem` (`self.NPCData`) (`KismetMathLibrary.RandomIntegerInRange` 0 (- (`KismetArrayLibrary.Array_Length` (`self.NPCData`)) 1))) null)
      (`/Engine/EditorBlueprintResources/StandardMacros.IncrementInt` (`self.Current NPCS`)))))

(fn `UnregisterNPC`
  (params (NPC :type "/Game/Blueprints/NPC/BP_NPC Object Reference"))
  (`KismetArrayLibrary.Array_RemoveItem` (`self.ActiveNPCs`) (`GameplayStatics.GetObjectClass` NPC)))

(fn `UserConstructionScript`)