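; BP_RegularNPC is a child Blueprint for a regular NPC, with events for interaction, sitting at a table and finishing an order.
; It adds no logic of its own: BeginPlay, Tick, Interactable, FinishOrder, SitinTable and the construction script all forward to the parent class.
; FinishOrder passes its success flag and table ID through unchanged, and the overlap event is a disabled stub.
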(event `self.ReceiveBeginPlay`
  (`parent.ReceiveBeginPlay`))

(event `self.ReceiveTick`
  (params (DeltaSeconds :type "Float (single-precision)"))
  (`parent.ReceiveTick` DeltaSeconds))

(event `/Game/ThirdPerson/Blueprints/BPI_Interactable.Interactable`
  (params (Player :type "/Game/ThirdPerson/Blueprints/BP_ThirdPersonCharacter Object Reference"))
  (`parent.Interactable` null))

(event `self.Finish Order`
  (params (IsSucess :type Boolean) (TableId :type Integer))
  (`parent.Finish Order` IsSucess TableId))

(event `self.Sit in table`
  (`parent.Sit in table`))

(fn `UserConstructionScript`
  (`parent.UserConstructionScript`))