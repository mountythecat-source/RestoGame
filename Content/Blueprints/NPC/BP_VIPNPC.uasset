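; VIP customer NPC Blueprint, a child of a parent NPC class that handles interaction, sitting at a table and finishing orders.
; Most events simply forward to the parent, while ResetTimer fails the current table's order through FinishOrder.
; UpdateTimer and SetTimer are empty, and the local queue and seat countdown logic, including progress widget updates, spawner unregistering and self-destruction, is disconnected and never runs.
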(event `self.ReceiveBeginPlay`
  (`parent.ReceiveBeginPlay`))

(event `self.UpdateTimer`)

(event `self.ReceiveTick`
  (params (DeltaSeconds :type "Float (single-precision)"))
  (`parent.ReceiveTick` DeltaSeconds))

(event `/Game/ThirdPerson/Blueprints/BPI_Interactable.Interactable`
  (params (Player :type "/Game/ThirdPerson/Blueprints/BP_ThirdPersonCharacter Object Reference"))
  (`parent.Interactable` null))

(event `self.Sit in table`
  (`parent.Sit in table`))

(event `self.Set Timer`)

(event `self.ResetTimer`
  (`self.Finish Order` false (`/Game/Blueprints/DiningRoom/BP_Table.TableID` (`self.BP Table`))))

(event `self.Finish Order`
  (params (IsSucess :type Boolean) (TableId :type Integer))
  (`parent.Finish Order` IsSucess TableId))

(fn `UserConstructionScript`
  (`parent.UserConstructionScript`))